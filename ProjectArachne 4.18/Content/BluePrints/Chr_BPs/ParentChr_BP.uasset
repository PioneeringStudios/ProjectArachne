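; Parent third-person shooter character handling movement, crouch, over-the-shoulder aiming, three weapon slots and empty use/skill functions for child characters.
; Tick eases the camera, sets walk speed, rebuilds the aim-only HUD and counts down reload timers.
; Weapon switches copy slot stats into one ActiveWeapon component, which drives line-trace firing with sound and particles, without damage.
; Pressing Reload again mid-reload attempts a timed fast reload, penalizing a miss.
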(event `self.ReceiveBeginPlay`)

(event `self.ReceiveTick`
  (params (DeltaSeconds :type "Float (single-precision)"))
  (set `self.Time` DeltaSeconds)
  (`|ExecutionSequence`
    (:`then_0`
      (`self.SetCameraAim`)
      (`self.SetMoveSpeed`))
    (:`then_1`
      (`self.SetHUDMode`))
    (:`then_2`
      (if (`self.IsReloading`)
        (if (> (`self.Timer_IsReloading`) 0.0)
          (set `self.Timer_IsReloading` (- (`self.Timer_IsReloading`) (`self.Time`)))
          (else
            (set `self.Timer_IsinAnimation` 0.0)
            (set `self.IsReloading` false)
            (`self.ReloadGun`)))))
    (:`then_3`
      (if (`self.IsInAnimation`)
        (if (> (`self.Timer_IsinAnimation`) 0.0)
          (set `self.Timer_IsinAnimation` (- (`self.Timer_IsinAnimation`) (`self.Time`)))
          (else
            (set `self.IsInAnimation` false)))))))

(event `InputAction|Jog`
  (params (Key :type "Key Structure"))
  ;[1 1 1] Listener to input(key) JOG, do cases and set JOG
  (:`Pressed`
    (set `self.JogPressed` true)
    (set `self.CrouchPressed` false)
    (set `self.ShouldTriggerCrouch` true))
  (:`Released`
    (set `self.JogPressed` false)))

(event `InputAction|Crouch`
  (params (Key :type "Key Structure"))
  ;[1 1 1] Listener to input(key) CROUCH, do cases and set CROUCH
  (:`Pressed`
    (set `self.ShouldTriggerCrouch` false)
    (set `self.CrouchPressed` true)
    (set `self.JogPressed` false))
  (:`Released`
    (set `self.ShouldTriggerCrouch` true)
    (set `self.CrouchPressed` false)))

(event `InputAction|Toggle Crouch`
  (params (Key :type "Key Structure"))
  ;[1 1 1] Listener to input(key) TOGGLE CROUCH, do cases and set CROUCH
  (:`Pressed`
    (if (`self.ShouldTriggerCrouch`) :!label _label
      (set `self.CrouchPressed` true)
      (set `self.ShouldTriggerCrouch` false)
      (set `self.JogPressed` false)
      (else
        (set `self.CrouchPressed` false)
        (set `self.ShouldTriggerCrouch` true)))))

(event `InputAction|Jump`
  (params (Key :type "Key Structure"))
  (bind _charactermovement (`self.CharacterMovement`))
  (bind _isaiming (`self.IsAiming`))
  ;[1 1 1] Listener to input(key) JUMP, do cases and set JUMP
  (:`Pressed`
    (if (`NavMovementComponent.IsFlying` (`self.CharacterMovement`))
      _
      (elif (`self.DisableMovement`)
        _
        (elif (`self.CrouchPressed`)
          (goto _label)
          (else
            (if (> (`KismetMathLibrary.VSize` (`MovementComponent.Velocity` (`self.CharacterMovement`))) 0.0)
              (`self.Jump`)
              (if _isaiming
                (set `CharacterMovementComponent.JumpZVelocity` 210.0 _charactermovement)
                (else
                  (set `CharacterMovementComponent.JumpZVelocity` 365.0 _charactermovement)))
              (else
                (`self.Jump`)
                (if _isaiming
                  (set `CharacterMovementComponent.JumpZVelocity` 200.0 _charactermovement)
                  (else
                    (set `CharacterMovementComponent.JumpZVelocity` 340.0 _charactermovement)))))
            (set `self.JumpPressed` true))))))
  (:`Released`
    (set `self.JumpPressed` false)))

(event `InputAction|Shoot`
  (params (Key :type "Key Structure"))
  ;[1 1 1] Listener to input(key) SHOOT, do cases and do SHOOT
  (:`Pressed`
    (if (not (`self.IsInAnimation`))
      (`self.Shooting`))))

(event `InputAction|Aim`
  (params (Key :type "Key Structure"))
  ;[1 1 1] Listener to input(key) AIM, do cases and do AIM
  (:`Pressed`
    (set `self.IsAiming` true))
  (:`Released`
    (set `self.IsAiming` false)))

(event `InputAxis|Turn`
  (params (AxisValue :type "Float (single-precision)"))
  ;[1 1 1] Input for movement and view.
  (`self.AddControllerYawInput` AxisValue))

(event `InputAxis|LookUp`
  (params (AxisValue :type "Float (single-precision)"))
  ;[1 1 1] Input for movement and view.
  (`self.AddControllerPitchInput` AxisValue))

(event `InputAxis|MoveForward`
  (params (AxisValue :type "Float (single-precision)"))
  ;[1 1 1] Input for movement and view.
  (if (not (`self.DisableMovement`))
    (`self.AddMovementInput` (`KismetMathLibrary.GetForwardVector` (`KismetMathLibrary.MakeRotator` 0.0 0.0 (.yaw (`self.GetControlRotation`)))) AxisValue)))

(event `InputAxis|MoveRight`
  (params (AxisValue :type "Float (single-precision)"))
  ;[1 1 1] Input for movement and view.
  (if (not (`self.DisableMovement`))
    (`self.AddMovementInput` (`KismetMathLibrary.GetRightVector` (`KismetMathLibrary.MakeRotator` 0.0 0.0 (.yaw (`self.GetControlRotation`)))) AxisValue)))

(event `InputAction|WeaponMain`
  (params (Key :type "Key Structure"))
  ;[1 1 1] input for Main weapon + change active weapon
  (:`Pressed`
    (if (not (`self.IsInAnimation`))
      (`self.SaveOldGun`)
      (set `self.ActiveGun` 1)
      (`self.ChangeToNewGun`))))

(event `InputAction|WeaponSub`
  (params (Key :type "Key Structure"))
  ;[1 1 1] input for sub weapon + change active weapon
  (:`Pressed`
    (if (not (`self.IsInAnimation`))
      (`self.SaveOldGun`)
      (set `self.ActiveGun` 2)
      (`self.ChangeToNewGun`))))

(event `InputAction|WeaponMelee`
  (params (Key :type "Key Structure"))
  ;[1 1 1] input for melee weapon + change active weapon
  (:`Pressed`
    (if (not (`self.IsInAnimation`))
      (`self.SaveOldGun`)
      (set `self.ActiveGun` 3)
      (`self.ChangeToNewGun`))))

(event `InputAction|WeaponNext`
  (params (Key :type "Key Structure"))
  ;[1 1 1] input for weapon next + change active weapon
  (:`Pressed`
    (if (not (`self.IsInAnimation`))
      (`self.SaveOldGun`)
      (bind _output_get (set `self.ActiveGun` (+ (`self.ActiveGun`) 1)))
      (if (> _output_get 3)
        (set `self.ActiveGun` 1))
      (`self.ChangeToNewGun`))))

(event `InputAction|WeaponPrevious`
  (params (Key :type "Key Structure"))
  ;[1 1 1] input for weapon previous + change active weapon
  (:`Pressed`
    (if (not (`self.IsInAnimation`))
      (`self.SaveOldGun`)
      (bind _output_get (set `self.ActiveGun` (- (`self.ActiveGun`) 1)))
      (if (< _output_get 1)
        (set `self.ActiveGun` 3))
      (`self.ChangeToNewGun`))))

(event `InputAction|Reload`
  (params (Key :type "Key Structure"))
  (bind _activeweapon (`self.ActiveWeapon`))
  ;[1 1 1] input for reload gun
  (:`Pressed`
    (if (`self.IsReloading`)
      (`self.ReloadShortcut`)
      (elif (`self.IsInAnimation`)
        _
        (elif (!= (`self.ActiveGun`) 3)
          (if (and (> (`/Game/BluePrints/Chr_BPs/Active_Gun_BP.Actual_Ammo_Amount` _activeweapon) 0) (< (`/Game/BluePrints/Chr_BPs/Active_Gun_BP.Actual_Clip_Amount` _activeweapon) (`/Game/BluePrints/Chr_BPs/Active_Gun_BP.Max_Clip_Amount` _activeweapon)))
            (`self.SetReloadGun`)))))))

(event `InputAction|Use`
  (params (Key :type "Key Structure"))
  ;[1 1 1] input for using object
  (:`Pressed`
    (if (`self.IsInAnimation`)
      _
      (elif (not (`self.IsAiming`))
        (`self.UseActivate`)))))

(event `InputAction|SkillPrimary`
  (params (Key :type "Key Structure"))
  ;[1 1 1] input for Primary skill
  (:`Pressed`
    (if (not (`self.IsInAnimation`))
      (`self.UsePrimarySkill`))))

(event `InputAction|SkillSecondary`
  (params (Key :type "Key Structure"))
  ;[1 1 1] input for Secondary skill
  (:`Pressed`
    (if (not (`self.IsInAnimation`))
      (`self.UseSecondarySkill`))))

(event `InputAction|SkillQuantity`
  (params (Key :type "Key Structure"))
  ;[1 1 1] input for Quantity skill
  (:`Pressed`
    (if (not (`self.IsInAnimation`))
      (`self.UseQuantitySkill`))))

(event `InputAction|SkillUltimate`
  (params (Key :type "Key Structure"))
  ;[1 1 1] input for Ultimate skill
  (:`Pressed`
    (if (not (`self.IsInAnimation`))
      (`self.UseUltimateSkill`))))

(fn `ChangeToNewGun`
  (bind _activeweapon (`self.ActiveWeapon`))
  (bind _activeweapon_2 (`self.ActiveWeapon`))
  (bind _activeweapon_3 (`self.ActiveWeapon`))
  (if (== (`self.ActiveGun`) 1)
    (set `/Game/BluePrints/Chr_BPs/Active_Gun_BP.Actual_Clip_Amount` (`self.Actual_Main_Clip_Size`) _activeweapon_2)
    (set `/Game/BluePrints/Chr_BPs/Active_Gun_BP.IsSpread` (`self.MainIsSpread`) _activeweapon_2)
    (set `/Game/BluePrints/Chr_BPs/Active_Gun_BP.HUD` (`self.Main_HUD`) _activeweapon_2)
    (set `/Game/BluePrints/Chr_BPs/Active_Gun_BP.FireSound` (`self.Main_FireSound`) _activeweapon_2)
    (set `/Game/BluePrints/Chr_BPs/Active_Gun_BP.TouchSound` (`self.Main_TouchSound`) _activeweapon_2)
    (set `/Game/BluePrints/Chr_BPs/Active_Gun_BP.TouchParticle` (`self.Main_TouchParticle`) _activeweapon_2)
    (set `/Game/BluePrints/Chr_BPs/Active_Gun_BP.Max_Range` (`self.Main_RangeWeapon`) _activeweapon_2)
    (set `/Game/BluePrints/Chr_BPs/Active_Gun_BP.Actual_Ammo_Amount` (`self.Actual_Main_Ammo_Amount`) _activeweapon_2)
    (set `/Game/BluePrints/Chr_BPs/Active_Gun_BP.Max_Clip_Amount` (`self.Max_Main_Clip_Size`) _activeweapon_2)
    (set `/Game/BluePrints/Chr_BPs/Active_Gun_BP.ReloadTime` (`self.Main_ReloadTime`) _activeweapon_2)
    (elif (== (`self.ActiveGun`) 2)
      (set `/Game/BluePrints/Chr_BPs/Active_Gun_BP.Actual_Clip_Amount` (`self.Actual_Sub_Clip_Size`) _activeweapon_3)
      (set `/Game/BluePrints/Chr_BPs/Active_Gun_BP.IsSpread` (`self.SubIsSpread`) _activeweapon_3)
      (set `/Game/BluePrints/Chr_BPs/Active_Gun_BP.HUD` (`self.Sub_HUD`) _activeweapon_3)
      (set `/Game/BluePrints/Chr_BPs/Active_Gun_BP.FireSound` (`self.Sub_FireSound`) _activeweapon_3)
      (set `/Game/BluePrints/Chr_BPs/Active_Gun_BP.TouchSound` (`self.Sub_TouchSound`) _activeweapon_3)
      (set `/Game/BluePrints/Chr_BPs/Active_Gun_BP.TouchParticle` (`self.Sub_TouchParticle`) _activeweapon_3)
      (set `/Game/BluePrints/Chr_BPs/Active_Gun_BP.Max_Range` (`self.Sub_RangeWeapon`) _activeweapon_3)
      (set `/Game/BluePrints/Chr_BPs/Active_Gun_BP.Actual_Ammo_Amount` (`self.Actual_Sub_Ammo_Amount`) _activeweapon_3)
      (set `/Game/BluePrints/Chr_BPs/Active_Gun_BP.Max_Clip_Amount` (`self.Max_Sub_Clip_Size`) _activeweapon_3)
      (set `/Game/BluePrints/Chr_BPs/Active_Gun_BP.ReloadTime` (`self.Sub_ReloadTime`) _activeweapon_3)
      (elif (== (`self.ActiveGun`) 3)
        (set `/Game/BluePrints/Chr_BPs/Active_Gun_BP.Actual_Clip_Amount` -1 _activeweapon)
        (set `/Game/BluePrints/Chr_BPs/Active_Gun_BP.IsSpread` false _activeweapon)
        (set `/Game/BluePrints/Chr_BPs/Active_Gun_BP.HUD` (`self.Melee_HUD`) _activeweapon)
        (set `/Game/BluePrints/Chr_BPs/Active_Gun_BP.FireSound` (`self.Melee_FireSound`) _activeweapon)
        (set `/Game/BluePrints/Chr_BPs/Active_Gun_BP.TouchSound` (`self.Melee_TouchSound`) _activeweapon)
        (set `/Game/BluePrints/Chr_BPs/Active_Gun_BP.TouchParticle` (`self.Melee_TouchParticle`) _activeweapon)
        (set `/Game/BluePrints/Chr_BPs/Active_Gun_BP.Max_Range` (`self.Melee_RangeWeapon`) _activeweapon)
        (set `/Game/BluePrints/Chr_BPs/Active_Gun_BP.Actual_Ammo_Amount` 0 _activeweapon)
        (set `/Game/BluePrints/Chr_BPs/Active_Gun_BP.Max_Clip_Amount` 0 _activeweapon)
        (set `/Game/BluePrints/Chr_BPs/Active_Gun_BP.ReloadTime` 0.0 _activeweapon)))))

(fn `ReloadGun`
  (bind _activeweapon (`self.ActiveWeapon`))
  (bind _activeweapon_2 (`self.ActiveWeapon`))
  (bind _activeweapon_3 (`self.ActiveWeapon`))
  (bind _activeweapon_4 (`self.ActiveWeapon`))
  (bind _returnvalue (- (`/Game/BluePrints/Chr_BPs/Active_Gun_BP.Actual_Ammo_Amount` _activeweapon) (- (`/Game/BluePrints/Chr_BPs/Active_Gun_BP.Max_Clip_Amount` _activeweapon) (`/Game/BluePrints/Chr_BPs/Active_Gun_BP.Actual_Clip_Amount` _activeweapon))))
  (if (< (- (`/Game/BluePrints/Chr_BPs/Active_Gun_BP.Max_Clip_Amount` _activeweapon_4) (`/Game/BluePrints/Chr_BPs/Active_Gun_BP.Actual_Clip_Amount` _activeweapon_4)) (`/Game/BluePrints/Chr_BPs/Active_Gun_BP.Actual_Ammo_Amount` _activeweapon_4))
    (switch `int` (`self.ActiveGun`)
      (:`1`
        (set `self.Actual_Main_Ammo_Amount` _returnvalue))
      (:`2`
        (set `self.Actual_Sub_Ammo_Amount` _returnvalue)))
    (set `/Game/BluePrints/Chr_BPs/Active_Gun_BP.Actual_Ammo_Amount` _returnvalue _activeweapon_2)
    (set `/Game/BluePrints/Chr_BPs/Active_Gun_BP.Actual_Clip_Amount` (`/Game/BluePrints/Chr_BPs/Active_Gun_BP.Max_Clip_Amount` _activeweapon_2) _activeweapon_2)
    (else
      (set `/Game/BluePrints/Chr_BPs/Active_Gun_BP.Actual_Clip_Amount` (+ (`/Game/BluePrints/Chr_BPs/Active_Gun_BP.Actual_Clip_Amount` _activeweapon_3) (`/Game/BluePrints/Chr_BPs/Active_Gun_BP.Actual_Ammo_Amount` _activeweapon_3)) _activeweapon_3)
      (set `/Game/BluePrints/Chr_BPs/Active_Gun_BP.Actual_Ammo_Amount` 0 (`self.ActiveWeapon`))
      (switch `int` (`self.ActiveGun`)
        (:`1`
          (set `self.Actual_Main_Ammo_Amount` 0))
        (:`2`
          (set `self.Actual_Sub_Ammo_Amount` 0))))))

(fn `ReloadShortcut`
  (bind _returnvalue (+ (`self.Timer_IsReloading`) 1.0))
  (if (`self.TriedFastReload`)
    _
    (elif (`KismetMathLibrary.InRange_FloatFloat` (`self.Timer_IsReloading`) (/ (* (`/Game/BluePrints/Chr_BPs/Active_Gun_BP.ReloadTime` (`self.ActiveWeapon`)) 50.0) 100.0) (/ (* (`/Game/BluePrints/Chr_BPs/Active_Gun_BP.ReloadTime` (`self.ActiveWeapon`)) 90.0) 100.0))
      (set `self.Timer_IsReloading` 0.0)
      (set `self.Timer_IsinAnimation` 0.0)
      (else
        (set `self.Timer_IsReloading` _returnvalue)
        (set `self.Timer_IsinAnimation` _returnvalue)
        (set `self.TriedFastReload` true)))))

(fn `SaveOldGun`
  (bind _actual_clip_amount (`/Game/BluePrints/Chr_BPs/Active_Gun_BP.Actual_Clip_Amount` (`self.ActiveWeapon`)))
  (if (== (`self.ActiveGun`) 1)
    (set `self.Actual_Main_Clip_Size` _actual_clip_amount)
    (elif (== (`self.ActiveGun`) 2)
      (set `self.Actual_Sub_Clip_Size` _actual_clip_amount))))

(fn `SetCameraAim`
  (bind _camera_loc (`self.Camera Loc`))
  (bind _time (`self.Time`))
  (bind _camera_loc_2 (`self.Camera Loc`))
  (bind _time_2 (`self.Time`))
  (bind _relativelocation (`SceneComponent.RelativeLocation` _camera_loc_2))
  (bind _relativelocation_2 (`SceneComponent.RelativeLocation` _camera_loc))
  ;[1 1 1] Get If Aiming, Change Camera Pos with lerp
  (if (`self.IsAiming`)
    (set `SpringArmComponent.TargetArmLength` (`KismetMathLibrary.FInterpTo` (`SpringArmComponent.TargetArmLength` _camera_loc) 20.0 (`self.Time`) 3.0) _camera_loc)
    (if (`self.CrouchPressed`)
      (`SceneComponent.K2_SetRelativeLocation` _camera_loc (`KismetMathLibrary.VInterpTo` _relativelocation_2 (0.0 50.0 35.0) _time 3.0) true false)
      (else
        (`SceneComponent.K2_SetRelativeLocation` _camera_loc (`KismetMathLibrary.VInterpTo` _relativelocation_2 (0.0 45.0 75.0) _time 3.0) true false)))
    (else
      (set `SpringArmComponent.TargetArmLength` (`KismetMathLibrary.FInterpTo` (`SpringArmComponent.TargetArmLength` _camera_loc_2) 60.0 (`self.Time`) 3.0) _camera_loc_2)
      (if (`self.CrouchPressed`)
        (`SceneComponent.K2_SetRelativeLocation` _camera_loc_2 (`KismetMathLibrary.VInterpTo` _relativelocation (0.0 50.0 35.0) _time_2 3.0) true false)
        (else
          (`SceneComponent.K2_SetRelativeLocation` _camera_loc_2 (`KismetMathLibrary.VInterpTo` _relativelocation (0.0 50.0 80.0) _time_2 3.0) true false))))))

(fn `SetHUDMode`
  (bind _activeweapon (`self.ActiveWeapon`))
  (`WidgetLayoutLibrary.RemoveAllWidgets`)
  (if (`self.IsAiming`)
    (bind _returnvalue (`|CreateWidget` (`/Game/BluePrints/Chr_BPs/Active_Gun_BP.HUD` (`self.ActiveWeapon`))))
    (bind _ashud (cast `/Game/GUI/HUD` _returnvalue))
    (`TextBlock.SetText` (`/Game/GUI/HUD.Ammo` _ashud) (`KismetTextLibrary.Conv_IntToText` (`/Game/BluePrints/Chr_BPs/Active_Gun_BP.Actual_Ammo_Amount` _activeweapon)))
    (`TextBlock.SetText` (`/Game/GUI/HUD.ClipSize` _ashud) (`KismetTextLibrary.Conv_IntToText` (`/Game/BluePrints/Chr_BPs/Active_Gun_BP.Actual_Clip_Amount` _activeweapon)))
    (`TextBlock.SetText` (`/Game/GUI/HUD.TypeWeapon` _ashud) (`KismetTextLibrary.Conv_IntToText` (`self.ActiveGun`)))
    (if (`self.TriedFastReload`)
      (bind _hint (`/Game/GUI/HUD.Hint` _ashud))
      (`TextBlock.SetText` _hint "" :!label _label)
      (elif (`KismetMathLibrary.InRange_FloatFloat` (`self.Timer_IsReloading`) (/ (* (`/Game/BluePrints/Chr_BPs/Active_Gun_BP.ReloadTime` (`self.ActiveWeapon`)) 50.0) 100.0) (/ (* (`/Game/BluePrints/Chr_BPs/Active_Gun_BP.ReloadTime` (`self.ActiveWeapon`)) 90.0) 100.0))
        (`TextBlock.SetText` _hint "FAST RELOAD !")
        (else
          (goto _label))))
    (`UserWidget.AddToViewport` _returnvalue 0)))

(fn `SetMoveSpeed`
  (bind _charactermovement (`self.CharacterMovement`))
  (bind _isaiming (`self.IsAiming`))
  (if (`self.JogPressed`)
    (if _isaiming
      (set `CharacterMovementComponent.MaxWalkSpeed` 102.5 _charactermovement)
      (else
        (set `CharacterMovementComponent.MaxWalkSpeed` 1000.0 _charactermovement)))
    (elif (`self.CrouchPressed`)
      (if _isaiming
        (set `CharacterMovementComponent.MaxWalkSpeed` 90.0 _charactermovement)
        (else
          (set `CharacterMovementComponent.MaxWalkSpeed` 180.0 _charactermovement)))
      (elif _isaiming
        (set `CharacterMovementComponent.MaxWalkSpeed` 102.5 _charactermovement)
        (else
          (set `CharacterMovementComponent.MaxWalkSpeed` 205.0 _charactermovement))))))

(fn `SetReloadGun`
  (bind _reloadtime (`/Game/BluePrints/Chr_BPs/Active_Gun_BP.ReloadTime` (`self.ActiveWeapon`)))
  (set `self.TriedFastReload` false)
  (set `self.Timer_IsReloading` _reloadtime)
  (set `self.Timer_IsinAnimation` _reloadtime)
  (set `self.IsInAnimation` true)
  (set `self.IsReloading` true))

(fn `SetUpGun`
  ;[1 1 1] Set up gun to be Main Gun
  (bind _returnvalue (`AddComponent|NODE_AddActive_Gun_BP-8` :`Actual_Clip_Amount` (`self.Actual_Main_Clip_Size`) :`Max_Clip_Amount` (`self.Max_Main_Clip_Size`) :`Actual_Ammo_Amount` (`self.Actual_Main_Ammo_Amount`) :`ReloadTime` (`self.Main_ReloadTime`) :`IsSpread` (`self.MainIsSpread`) :`HUD` (`self.Main_HUD`) :`FireSound` (`self.Main_FireSound`) :`TouchSound` (`self.Main_TouchSound`) :`TouchParticle` (`self.Main_TouchParticle`) :`Max_Range` (`self.Main_RangeWeapon`)))
  (set `self.ActiveWeapon` _returnvalue))

(fn `Shooting`
  (bind _returnvalue (`self.K2_GetActorLocation`))
  (bind _activeweapon (`self.ActiveWeapon`))
  (bind _returnvalue_2 (`KismetMathLibrary.MakeVector` (.x _returnvalue) (.y _returnvalue) (+ (.z _returnvalue) 20.0)))
  ;[1 1 1] Listener to input(key) SHOOT, do cases and do SHOOT
  (if (== (`self.ActiveGun`) 3)
    (`GameplayStatics.PlaySoundAtLocation` (`/Game/BluePrints/Chr_BPs/Active_Gun_BP.FireSound` (`self.ActiveWeapon`)) _returnvalue :!label _label)
    (bind _outhit (`KismetSystemLibrary.LineTraceSingle` :`Start` _returnvalue_2 :`End` (+ _returnvalue_2 (* (`KismetMathLibrary.GetForwardVector` (`self.GetControlRotation`)) (`/Game/BluePrints/Chr_BPs/Active_Gun_BP.Max_Range` (`self.ActiveWeapon`)))) :`TraceChannel` "TraceTypeQuery1" :`DrawDebugType` "ForDuration"))
    (bind (_bblockinghit _binitialoverlap _time _distance _location) (`GameplayStatics.BreakHitResult` _outhit))
    ;;[1 1 1] To add : PARTICLES + SOUNDS AT END LOC OF RAYCAST IF ANY
    (`GameplayStatics.SpawnEmitterAtLocation` (`/Game/BluePrints/Chr_BPs/Active_Gun_BP.TouchParticle` (`self.ActiveWeapon`)) _location)
    (`GameplayStatics.PlaySoundAtLocation` (`/Game/BluePrints/Chr_BPs/Active_Gun_BP.TouchSound` (`self.ActiveWeapon`)) _location)
    (elif (> (`/Game/BluePrints/Chr_BPs/Active_Gun_BP.Actual_Clip_Amount` (`self.ActiveWeapon`)) 0)
      ;[1 1 1] Remove 1 bullet in actual clip
      (set `/Game/BluePrints/Chr_BPs/Active_Gun_BP.Actual_Clip_Amount` (- (`/Game/BluePrints/Chr_BPs/Active_Gun_BP.Actual_Clip_Amount` _activeweapon) 1) _activeweapon)
      (goto _label)
      (else
        (`self.ReloadGun`)))))

(fn `UseActivate`)

(fn `UsePrimarySkill`)

(fn `UseQuantitySkill`)

(fn `UserConstructionScript`)

(fn `UseSecondarySkill`)

(fn `UseUltimateSkill`)