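; Assault character Blueprint, a child class that sets up its weapon loadout and hooks into the four-skill system.
; On BeginPlay it spawns three test gun actors at the mesh transform and registers them as main, sub and melee weapons, passing projectile spawn points for the first two.
; Each skill event calls its parent, commented as handling cooldown or removal, then a class-specific skill function, all four of which are still empty stubs.
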(event `self.UsePrimarySkill`
  ;[1 1 1] call parents to start CD/remove, then call class function to do special power
  (`parent.UsePrimarySkill`)
  (`self.SkillPrim`))

(event `self.UseSecondarySkill`
  ;[1 1 1] call parents to start CD/remove, then call class function to do special power
  (`parent.UseSecondarySkill`)
  (`self.SkillSec`))

(event `self.UseQuantitySkill`
  ;[1 1 1] call parents to start CD/remove, then call class function to do special power
  (`parent.UseQuantitySkill`)
  (`self.SkillQty`))

(event `self.UseUltimateSkill`
  ;[1 1 1] call parents to start CD/remove, then call class function to do special power
  (`parent.UseUltimateSkill`)
  (`self.SkillUlt`))

(event `self.ReceiveBeginPlay`
  (bind _mesh (`self.Mesh`))
  (bind _returnvalue (`SceneComponent.K2_GetComponentToWorld` _mesh))
  (bind _returnvalue_2 (`|SpawnActorFromClass` "/Game/BluePrints/Chr_BPs/TEST_ACTOR_GUN.TEST_ACTOR_GUN_C" _returnvalue "Undefined" "OverrideRootScale" null null))
  (bind _returnvalue_3 (`|SpawnActorFromClass` "/Game/BluePrints/Chr_BPs/TEST_ACTOR_GUN1.TEST_ACTOR_GUN1_C" _returnvalue "Undefined" "OverrideRootScale" null null))
  (bind _returnvalue_4 (`|SpawnActorFromClass` "/Game/BluePrints/Chr_BPs/TEST_ACTOR_GUN2.TEST_ACTOR_GUN2_C" _returnvalue "Undefined" "OverrideRootScale" null null))
  (`self.SetPropertiesNewGun` _returnvalue_2 (`/Game/BluePrints/Chr_BPs/TEST_ACTOR_GUN.ProjectilePointSpawn` _returnvalue_2) _returnvalue_3 (`/Game/BluePrints/Chr_BPs/TEST_ACTOR_GUN1.ProjectilePointSpawn` _returnvalue_3) _returnvalue_4 _mesh))

(fn `SkillPrim`)

(fn `SkillQty`)

(fn `SkillSec`)

(fn `SkillUlt`)

(fn `UserConstructionScript`)