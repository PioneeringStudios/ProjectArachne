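; Game-instance-style Blueprint that manages menu screens and multiplayer sessions for hosting, browsing, joining and leaving games.
; A ChangeStates macro removes the outgoing state's widget, or destroys the session when leaving Playing, before show events lazily create and display theirs.
; Hosting opens SpaceStation as a listen server, while session, network and travel failures feed an error dialog that also destroys the session.
; Saved-settings loading is unwired, and SetSettings forces a fixed resolution.
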(event `Show Settings Screen`
  (bind _returnvalue (`GameplayStatics.GetPlayerController` 0))
  (bind _returnvalue_2 (`GameplayStatics.GetPlayerController` 0))
  (`self.IsCurrentState` "NewEnumerator1"
    (:`True`
      (`self.ChangeStates` "NewEnumerator8"
        (:`NewState`
          (`/Engine/EditorBlueprintResources/StandardMacros.IsValid` (`self.Settings`)
            (:`Is Valid`
              _)
            (:`Is Not Valid`
              (bind _returnvalue_3 (`|CreateWidget` "/Game/GUI/UMG/MainMenu/W_Settings.W_Settings_C" _returnvalue))
              (bind _output_get (set `self.Settings` _returnvalue_3))))
          (`UserWidget.AddToViewport` _output_get 0)
          (`Widget.SetVisibility` _output_get "Visible")
          (`WidgetBlueprintLibrary.SetInputMode_UIOnlyEx` _returnvalue _output_get))))
    (:`False`
      (`/Engine/EditorBlueprintResources/StandardMacros.IsValid` (`self.Settings`)
        (:`Is Valid`
          _)
        (:`Is Not Valid`
          (bind _returnvalue_4 (`|CreateWidget` "/Game/GUI/UMG/MainMenu/W_Settings.W_Settings_C" _returnvalue_2))
          (bind _output_get_2 (set `self.Settings` _returnvalue_4))))
      (`UserWidget.AddToViewport` _output_get_2 0)
      (`Widget.SetVisibility` _output_get_2 "Visible")
      (`WidgetBlueprintLibrary.SetInputMode_UIOnlyEx` _returnvalue_2 _output_get_2))))

(event `ShowLoadScreen`
  (bind _returnvalue (`GameplayStatics.GetPlayerController` 0))
  ;[1 1 1] Show Loading Screen when Transfering Maps
  (`self.ChangeStates` "NewEnumerator6"
    (:`NewState`
      (`/Engine/EditorBlueprintResources/StandardMacros.IsValid` (`self.Loading`)
        (:`Is Valid`
          _)
        (:`Is Not Valid`
          (bind _returnvalue_2 (`|CreateWidget` "/Game/GUI/UMG/MainMenu/W_LoadingScreen.W_LoadingScreen_C" _returnvalue))
          (bind _output_get (set `self.Loading` _returnvalue_2))))
      (`UserWidget.AddToViewport` _output_get 0)
      (`WidgetBlueprintLibrary.SetInputMode_UIOnlyEx` _returnvalue _output_get))))

(event `JoinFromServerListEvent`
  (params (searchResult :type "BlueprintSessionResult Structure"))
  ;[1 1 1] Join Sever Event
  (`self.ShowLoadScreen`)
  (`JoinSessionCallbackProxy.JoinSession` (`GameplayStatics.GetPlayerController` 0) searchResult
    (:`OnFailure`
      (`self.DisplayError` "Failed to join server!"))))

(event `ShowServerListEvent`
  (bind _returnvalue (`GameplayStatics.GetPlayerController` 0))
  ;[1 1 1] Show Server list when clicked from main menu
  (`self.ChangeStates` "NewEnumerator4"
    (:`NewState`
      (`/Engine/EditorBlueprintResources/StandardMacros.IsValid` (`self.ServerList`)
        (:`Is Valid`
          _)
        (:`Is Not Valid`
          (bind _returnvalue_2 (`|CreateWidget` "/Game/GUI/UMG/MainMenu/W_ServerList.W_ServerList_C" _returnvalue))
          (bind _output_get (set `self.ServerList` _returnvalue_2))))
      (`UserWidget.AddToViewport` _output_get 0)
      (`WidgetBlueprintLibrary.SetInputMode_UIOnlyEx` _returnvalue _output_get))))

(event `ShowMainMenuEvent`
  (bind _returnvalue (`GameplayStatics.GetPlayerController` 0))
  ;[1 1 1] Show/Create MainMenu
  (`self.IsCurrentState` "NewEnumerator2"
    (:`True`
      (`GameplayStatics.OpenLevel` "MainMenu"))
    (:`False`
      (`self.ChangeStates` "NewEnumerator1"
        (:`NewState`
          (`/Engine/EditorBlueprintResources/StandardMacros.IsValid` (`self.MainMenu`)
            (:`Is Valid`
              _)
            (:`Is Not Valid`
              (bind _returnvalue_2 (`|CreateWidget` "/Game/GUI/UMG/MainMenu/W_MainMenu.W_MainMenu_C" _returnvalue))
              (bind _output_get (set `self.MainMenu` _returnvalue_2))))
          (`WidgetBlueprintLibrary.SetInputMode_UIOnlyEx` _returnvalue _output_get)
          (`UserWidget.AddToViewport` _output_get 0))))))

(event `HostGameEvent`
  ;[1 1 1] Host Game Session - Called from Main Menu Widget
  (`self.ShowLoadScreen`)
  (`CreateSessionCallbackProxy.CreateSession` (`GameplayStatics.GetPlayerController` 0) 3 (`self.b_EnableLan`)
    (:`OnSuccess`
      (`KismetSystemLibrary.PrintString` "SessionCreated")
      (`GameplayStatics.OpenLevel` "SpaceStation" true "listen"))
    (:`OnFailure`
      (`self.DisplayError` "Error: Could not create session"))))

(event `LeaveSettings`
  ;[1 1 1] Leave setting to get back in game
  (`self.ChangeStates` "NewEnumerator2"
    (:`NewState`
      (`Widget.SetVisibility` (`self.Settings`) "Hidden"))))

(event `DestroySessionCaller`
  ;[1 1 1] Destroy Session
  (`DestroySessionCallbackProxy.DestroySession` (`GameplayStatics.GetPlayerController` 0)))

(event `self.HandleNetworkError`
  (params (FailureType :type "ENetworkFailure Enum" :default "NetDriverAlreadyExists") (bIsServer :type Boolean))
  ;[1 1 1] Catch Netcode Errors
  (if (not bIsServer)
    (`self.DisplayError` (`self.toNetcodeErrorString` FailureType))))

(event `LeaveGame`
  (params (LeaveSession :type Boolean))
  ;[1 1 1] Leave game, destroy sess and show menu
  (if LeaveSession
    (`self.ChangeStates` "NewEnumerator0"
      (:`NewState`
        (`self.DestroySessionCaller`)
        (`self.ShowMainMenuEvent`)))
    (else
      (`KismetSystemLibrary.QuitGame` (`GameplayStatics.GetPlayerController` 0) "Quit"))))

(event `self.HandleTravelError`
  (params (FailureType :type "ETravelFailure Enum" :default "NoLevel"))
  ;[1 1 1] Catch Travel Errors
  (`self.DisplayError` (`self.toTravelErrorString` FailureType)))

(fn `BeginPlay_ShowMainMenu`
  ;[1 1 1] Show main menu when restart or launching
  (`self.IsCurrentState` "NewEnumerator0"
    (:`True`
      (`self.ShowMainMenuEvent`))))

(fn `CompareCurrentState`
  (params (State :type "/Game/BluePrints/MainMenu_BPs/E_GameState Enum" :default "NewEnumerator0"))
  (returns (Check :type Boolean))
  ;[1 1 1] Compare Input State to Variable State
  (return (`|EnumEquality` State (`self.currentState`))))

(fn `HideWidget`
  (params (WidgetRef :type "Widget Object Reference"))
  ;[1 1 1] Takes Widget off of Screen
  (`Widget.RemoveFromParent` WidgetRef))

(fn `SetSettings`
  (params (`Game Settings` :type "/Game/GUI/UMG/MainMenu/Settings/Settings_Save Object Reference"))
  (bind _assettings_save (cast `/Game/GUI/UMG/MainMenu/Settings/Settings_Save` `Game Settings`))
  (`KismetSystemLibrary.ExecuteConsoleCommand` "r.setRes 1920x1080f")
  (return))

(fn `StartPlayingState`
  (`self.ChangeStates` "NewEnumerator2"))

(fn `toNetcodeErrorString`
  (params (inerror :type "ENetworkFailure Enum" :default "NetDriverAlreadyExists"))
  (returns (errorout :type String))
  (switch `ENetworkFailure` inerror
    (:`NetDriverAlreadyExists`
      _)
    (:`NetDriverCreateFailure`
      _)
    (:`NetDriverListenFailure`
      _)
    (:`ConnectionLost`
      _)
    (:`ConnectionTimeout`
      (return "Error, connection timed out!"))
    (:`FailureReceived`
      _)
    (:`OutdatedClient`
      _)
    (:`OutdatedServer`
      _)
    (:`PendingConnectionFailure`
      _)
    (:`NetGuidMismatch`
      _)
    (:`NetChecksumMismatch`
      _))
  (return "Error, lost connection to host!"))

(fn `toTravelErrorString`
  (params (inerror :type "ETravelFailure Enum" :default "NoLevel"))
  (returns (errorout :type String))
  (return (`KismetStringLibrary.Concat_StrStr` "Error travelling maps due to:" (`|GetEnumeratorNameAsString` inerror))))