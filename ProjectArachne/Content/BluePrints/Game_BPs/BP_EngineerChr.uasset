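; Engineer hero character that spawns its three weapons on BeginPlay and implements class skills on top of parent cooldown handling.
; Primary toggles a timed taunt, secondary spawns a timed wall on authority, and the quantity skill throws a grenade.
; Ultimate spawns teleporters on authority, keeping two cross-linked by location and alternately replacing them.
; Passive trims primary and secondary cooldowns on "friendly"-tagged characters by a fraction of their maximum.
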(event `self.UsePrimarySkill`
  ;[1 1 1] call parents to start CD/remove, then call class function to do special power
  (`parent.usePrimarySkill`)
  (`self.useSkillPrimary`))

(event `self.UseSecondarySkill`
  ;[1 1 1] call parents to start CD/remove, then call class function to do special power
  (`parent.useSecondarySkill`)
  (`self.useSkillSecondary`))

(event `self.useQuantitySkill`
  ;[1 1 1] call parents to start CD/remove, then call class function to do special power
  (`parent.useQuantitySkill`)
  (`self.useSkillQty`))

(event `self.UseUltimateSkill`
  ;[1 1 1] call parents to start CD/remove, then call class function to do special power
  (`parent.useUltimateSkill`)
  (`self.useSkillUltimate`))

(event `self.spawnQtySkill`
  ;[1 1 1] call parents to start CD/remove, then call class function to do special power
  (`self.spawnMyQtySkill`))

(event `self.incrementPassiveSkill`
  ;[1 1 1] call parents to start CD/remove, then call class function to do special power
  (`self.incrementMyPassiveSkill`))

(event `self.deactivateSecSkill`
  ;[1 1 1] call parents to start CD/remove, then call class function to do special power
  (`self.deactivateMySecSkill`))

(event `self.deactivatePrimSkill`
  ;[1 1 1] call parents to start CD/remove, then call class function to do special power
  (`self.deactivateMyPrimSkill`))

(event `self.deactivateUltSkill`
  ;[1 1 1] call parents to start CD/remove, then call class function to do special power
  (`self.deactiveMyUltSkill`))

(event `self.ReceiveTick`
  (params (DeltaSeconds :type "Float (single-precision)"))
  (`parent.ReceiveTick` DeltaSeconds))

(event `self.ReceiveBeginPlay`
  (bind _returnvalue (`SceneComponent.K2_GetComponentToWorld` (`self.Mesh`)))
  (bind _returnvalue_2 (`|SpawnActorFromClass` "/Game/BluePrints/Game_BPs/Guns/TEST_ACTOR_GUN.TEST_ACTOR_GUN_C" _returnvalue "Undefined" "OverrideRootScale" null null))
  (bind _returnvalue_3 (`|SpawnActorFromClass` "/Game/BluePrints/Game_BPs/Guns/TEST_ACTOR_GUN1.TEST_ACTOR_GUN1_C" _returnvalue "Undefined" "OverrideRootScale" null null))
  (bind _returnvalue_4 (`|SpawnActorFromClass` "/Game/BluePrints/Game_BPs/Guns/TEST_ACTOR_GUN2.TEST_ACTOR_GUN2_C" _returnvalue "Undefined" "OverrideRootScale" null null))
  (`self.createBaseGun` _returnvalue_2 (`/Game/BluePrints/Game_BPs/Guns/TEST_ACTOR_GUN.ProjectilePointSpawn` _returnvalue_2) _returnvalue_3 (`/Game/BluePrints/Game_BPs/Guns/TEST_ACTOR_GUN1.ProjectilePointSpawn` _returnvalue_3) _returnvalue_4)
  (`parent.ReceiveBeginPlay`))

(fn `deactivateMyPrimSkill`
  (set `self.b_IsTaunting` false))

(fn `deactivateMySecSkill`)

(fn `deactiveMyUltSkill`)

(fn `incrementMyPassiveSkill`
  ;[1 1 1] Remove 20% of CD
  (bind _outactors (`GameplayStatics.GetAllActorsWithTag` "friendly"))
  (for _array_element _outactors
    (bind _asbp_parent_chr (cast `/Game/BluePrints/Game_BPs/BP_ParentChr` _array_element))
    (bind _flt_timerprimaryskill (`/Game/BluePrints/Game_BPs/BP_ParentChr.flt_timerPrimarySkill` _asbp_parent_chr))
    (if (> _flt_timerprimaryskill 0.0)
      (bind _returnvalue (- _flt_timerprimaryskill (/ (* (`/Game/BluePrints/Game_BPs/BP_ParentChr.MAX_TIMER_PRIMARY_SKILL` _asbp_parent_chr) 10.0) 100.0)))
      (if (< _returnvalue 0.0)
        (set `/Game/BluePrints/Game_BPs/BP_ParentChr.flt_timerPrimarySkill` 0.0 _asbp_parent_chr)
        (else
          (set `/Game/BluePrints/Game_BPs/BP_ParentChr.flt_timerPrimarySkill` _returnvalue _asbp_parent_chr)
          (bind _flt_timersecondaryskill (`/Game/BluePrints/Game_BPs/BP_ParentChr.flt_timerSecondarySkill` _asbp_parent_chr))
          (if (> _flt_timersecondaryskill 0.0) :!label _label
            (bind _returnvalue_2 (- _flt_timersecondaryskill (/ (* (`/Game/BluePrints/Game_BPs/BP_ParentChr.MAX_TIMER_SECONDARY_SKILL` _asbp_parent_chr) 10.0) 100.0)))
            (if (< _returnvalue_2 0.0)
              (set `/Game/BluePrints/Game_BPs/BP_ParentChr.flt_timerSecondarySkill` 0.0 _asbp_parent_chr)
              (else
                (set `/Game/BluePrints/Game_BPs/BP_ParentChr.flt_timerSecondarySkill` _returnvalue_2 _asbp_parent_chr))))))
      (else
        (goto _label)))))

(fn `PopulateTeleport`
  (params (int_nextTP :type Integer) (ref_engiUlt :type "/Game/BluePrints/Game_BPs/SkillsActors/A_EngiUlti Object Reference") (b_destroyOld :type Boolean))
  (bind _ulti_1 (`self.ulti_1`))
  (bind _ulti_2 (`self.ulti_2`))
  (switch `int` int_nextTP
    (:`1`
      (if b_destroyOld
        (`/Game/BluePrints/Game_BPs/SkillsActors/A_EngiUlti.DestroyTeleport` (`self.ulti_1`)))
      (bind _output_get (set `self.ulti_1` ref_engiUlt))
      (set `self.int_nextTeleportToPopulate` 2)
      (if (`KismetSystemLibrary.IsValid` _ulti_2)
        (set `/Game/BluePrints/Game_BPs/SkillsActors/A_EngiUlti.vec_secondTeleport` (`self.K2_GetActorLocation` _ulti_2) _output_get)
        (set `/Game/BluePrints/Game_BPs/SkillsActors/A_EngiUlti.vec_secondTeleport` (`self.K2_GetActorLocation` _output_get) _ulti_2)))
    (:`2`
      (if b_destroyOld
        (`/Game/BluePrints/Game_BPs/SkillsActors/A_EngiUlti.DestroyTeleport` (`self.ulti_2`)))
      (bind _output_get_2 (set `self.ulti_2` ref_engiUlt))
      (set `self.int_nextTeleportToPopulate` 1)
      (if (`KismetSystemLibrary.IsValid` _ulti_1)
        (set `/Game/BluePrints/Game_BPs/SkillsActors/A_EngiUlti.vec_secondTeleport` (`self.K2_GetActorLocation` _ulti_1) _output_get_2)
        (set `/Game/BluePrints/Game_BPs/SkillsActors/A_EngiUlti.vec_secondTeleport` (`self.K2_GetActorLocation` _output_get_2) _ulti_1)))))

(fn `spawnMyQtySkill`
  (bind _mesh (`self.Mesh`))
  (`|SpawnActorFromClass` (`self.RefQtySkillGrenade`) (`KismetMathLibrary.MakeTransform` (`SceneComponent.GetSocketLocation` _mesh "S_Active_Weapon") (`SceneComponent.GetSocketRotation` _mesh "S_Active_Weapon")) "Undefined" "OverrideRootScale" null null))

(fn `UserConstructionScript`)

(fn `useSkillPrimary`
  (set `self.flt_timerInUsePrimSkill` 5.0)
  (set `self.b_primSkillOn` true)
  (set `self.b_IsTaunting` true))

(fn `useSkillQty`
  (`self.PlayAnimMontage` "/Game/BluePrints/Game_BPs/Montage/MT_THROWGRENADE.MT_THROWGRENADE")
  (set `self.flt_timerIsinAction` 1.5)
  (set `self.b_triggerSpawnGrenade` true))

(fn `useSkillSecondary`
  (bind (_returnvalue_location _returnvalue_rotation _returnvalue_scale) (`KismetMathLibrary.BreakTransform` (`self.GetTransform`)))
  (`/Engine/EditorBlueprintResources/ActorMacros.Switch Has Authority`
    (:`Authority`
      (bind _returnvalue (`|SpawnActorFromClass` "/Game/BluePrints/Game_BPs/SkillsActors/A_EngiSec.A_EngiSec_C" (`KismetMathLibrary.MakeTransform` (+ _returnvalue_location (* (`SceneComponent.GetForwardVector` (`self.Mesh`)) 5.0)) _returnvalue_rotation _returnvalue_scale) "Undefined" "OverrideRootScale" null null))
      (`/Game/BluePrints/Game_BPs/SkillsActors/A_EngiSec.SetTimerWall` _returnvalue 5.0))))

(fn `useSkillUltimate`
  (`/Engine/EditorBlueprintResources/ActorMacros.Switch Has Authority`
    (:`Authority`
      (bind _returnvalue (`|SpawnActorFromClass` "/Game/BluePrints/Game_BPs/SkillsActors/A_EngiUlti.A_EngiUlti_C" (`SceneComponent.K2_GetComponentToWorld` (`/Game/BluePrints/Game_BPs/CBP_Active_Gun.WeaponArrow` (`self.ActiveWeapon`))) "Undefined" "OverrideRootScale" null null))
      (if (`KismetSystemLibrary.IsValid` (`self.ulti_1`))
        (if (`KismetSystemLibrary.IsValid` (`self.ulti_2`))
          (`self.PopulateTeleport` (`self.int_nextTeleportToPopulate`) _returnvalue true)
          (else
            (`self.PopulateTeleport` 2 _returnvalue)))
        (else
          (`self.PopulateTeleport` 1 _returnvalue))))))