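; Base Blueprint for interactive map assets that can be toggled on or off, with an optional timed auto-off.
; ActivateMapInteractive flips the state through TurnOnOff, which ignores requests while locked and calls DoOnActor or DoOffActor, empty hooks for children to override.
; Switching on passes the max timer value; when it is positive, Tick counts it down via TimerDecrease and switches the asset off on expiry.
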(event `self.ReceiveTick`
  (params (DeltaSeconds :type "Float (single-precision)"))
  (set `self.flt_delta` DeltaSeconds)
  (`self.timerDecrease`))

(fn `activateMapInteractive`
  (bind _b_onoff (`self.b_onOff`))
  (bind _returnvalue (not _b_onoff))
  (if _b_onoff
    (`self.turnOnOff` _returnvalue) ; if was on
    (else
      (`self.turnOnOff` _returnvalue (`self.flt_MAX_TIMER`)) ; if was off
    )))

(fn `doOffActor`)

(fn `doOnActor`)

(fn `timerDecrease`
  (if (`self.b_isTimer`)
    (if (> (`self.flt_timerOn`) 0.0)
      (set `self.flt_timerOn` (- (`self.flt_timerOn`) (`self.flt_delta`)))
      (else
        (`self.turnOnOff` false)))))

(fn `turnOnOff`
  (params (b_onOff :type Boolean) (flt_timerOn :type "Float (double-precision)" :default 0.0))
  (if (not (`self.b_lock`))
    (bind _output_get (set `self.b_onOff` b_onOff))
    (if _output_get
      (`self.doOnActor`)
      (if (> flt_timerOn 0.0)
        (set `self.b_isTimer` true)
        (set `self.flt_timerOn` flt_timerOn))
      (else
        (`self.doOffActor`)
        (if (`self.b_isTimer`)
          (set `self.b_isTimer` false))))))

(fn `UserConstructionScript`)