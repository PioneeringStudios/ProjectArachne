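; BP_Door_1 is an interactive map door that slides its left door mesh between open and closed positions.
; It extends the parent's on and off actor events to set a move flag.
; Each Tick eases the mesh toward the open or close arrow's world location, chosen by BOnOff, using a fixed-alpha, frame-rate-dependent lerp.
; The flag clears once the mesh is within tolerance of its target.
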(event `self.ReceiveTick`
  (params (DeltaSeconds :type "Float (single-precision)"))
  (`parent.ReceiveTick` DeltaSeconds)
  (`self.DoLerpToLoc`))

(event `self.doOnActor`
  (`parent.doOnActor`)
  (`self.DoorDoOnActor`))

(event `self.doOffActor`
  (`parent.doOffActor`)
  (`self.DoorDoOffActor`))

(fn `DoLerpToLoc`
  (bind _returnvalue (`SceneComponent.K2_GetComponentLocation` (`self.LeftArrowClosePos`)))
  (bind _returnvalue_2 (`SceneComponent.K2_GetComponentLocation` (`self.LeftDoorMesh`)))
  (bind _returnvalue_3 (`SceneComponent.K2_GetComponentLocation` (`self.LeftArrowOpenPos`)))
  (bind _returnvalue_4 (`SceneComponent.K2_GetComponentLocation` (`self.LeftDoorMesh`)))
  (if (`self.b_moveTo`)
    (if (`self.b_onOff`)
      (`SceneComponent.K2_SetWorldLocation` (`self.LeftDoorMesh`) (`KismetMathLibrary.VLerp` _returnvalue_4 _returnvalue_3 0.1) false false)
      (if (== _returnvalue_3 _returnvalue_4 :`ErrorTolerance` 0.001)
        (set `self.b_moveTo` false))
      (else
        (`SceneComponent.K2_SetWorldLocation` (`self.LeftDoorMesh`) (`KismetMathLibrary.VLerp` _returnvalue_2 _returnvalue 0.1) false false)
        (if (== _returnvalue _returnvalue_2 :`ErrorTolerance` 0.001)
          (set `self.b_moveTo` false))))))

(fn `DoorDoOffActor`
  (set `self.b_moveTo` true))

(fn `DoorDoOnActor`
  (set `self.b_moveTo` true))

(fn `UserConstructionScript`
  (`parent.UserConstructionScript`))