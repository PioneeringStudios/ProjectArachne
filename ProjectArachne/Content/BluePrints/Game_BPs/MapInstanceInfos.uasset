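; MapInstanceInfos is a map-level Blueprint that periodically spawns AI enemies or units on the server.
; Its authority-only Tick counts down a respawn timer, resetting it to a maximum on expiry.
; It then measures synchronous navigation path lengths from every AISpawner to every BP_ParentChr actor.
; A BP_AIs actor spawns at the arrow transform of the spawner with the shortest path to any character.
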(event `self.ReceiveTick`
  (params (DeltaSeconds :type "Float (single-precision)"))
  (`/Engine/EditorBlueprintResources/ActorMacros.Switch Has Authority`
    (:`Authority`
      (set `self.flt_Delta` DeltaSeconds)
      (if (<= (`self.flt_RespawnTimer`) 0.0)
        (`KismetSystemLibrary.PrintString` "respawn }")
        (set `self.flt_RespawnTimer` (`self.MAX_RESPAWN_TIMER`))
        (set `self.flt_LengthClosestSpawner` 99999.0) ; reset found closest amount
        (bind _outactors (`GameplayStatics.GetAllActorsOfClass` "/Game/BluePrints/Game_BPs/AIs/AISpawner.AISpawner_C"))
        (bind _outactors_2 (`GameplayStatics.GetAllActorsOfClass` "/Game/BluePrints/Game_BPs/BP_ParentChr.BP_ParentChr_C"))
        (for (_array_element _array_index) _outactors
          (for _array_element_2 _outactors_2
            (bind _returnvalue (`NavigationSystem.FindPathToActorSynchronously` (`SceneComponent.K2_GetComponentLocation` (`/Game/BluePrints/Game_BPs/AIs/AISpawner.Arrow` _array_element)) _array_element_2))
            (bind _returnvalue_2 (`NavigationPath.GetPathLength` _returnvalue))
            (if (< _returnvalue_2 (`self.flt_LengthClosestSpawner`))
              (set `self.flt_LengthClosestSpawner` _returnvalue_2)
              (set `self.int_IndexClosestSpawner` _array_index))))
        (`|SpawnActorFromClass` "/Game/BluePrints/Game_BPs/AIs/BP_AIs.BP_AIs_C" (`SceneComponent.K2_GetComponentToWorld` (`/Game/BluePrints/Game_BPs/AIs/AISpawner.Arrow` (`|GetArrayItem` _outactors (`self.int_IndexClosestSpawner`)))) "Undefined" "OverrideRootScale" null null)
        (else
          (set `self.flt_RespawnTimer` (- (`self.flt_RespawnTimer`) (`self.flt_Delta`))))))))

(fn `UserConstructionScript`)