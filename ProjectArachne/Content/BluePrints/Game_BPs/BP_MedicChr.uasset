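; Medic character that layers class skills over parent skill events and spawns three test weapons at BeginPlay.
; Primary fires a server-spawned heal projectile; quantity skill plays a throw montage, flagging a grenade later spawned by SpawnQtySkill.
; Secondary and ultimate both spawn the timed medic ultimate on the server, leaving the adrenaline-boost function unreached.
; Passive increment heals every "friendly"-tagged character by a percentage of max health, capped at max.
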(event `self.UsePrimarySkill`
  ;[1 1 1] call parents to start CD/remove, then call class function to do special power
  (`parent.usePrimarySkill`)
  (`self.useSkillPrimary`))

(event `self.UseSecondarySkill`
  ;[1 1 1] call parents to start CD/remove, then call class function to do special power
  (`parent.useSecondarySkill`)
  (`self.useSkillUltimate` :!label _label))

(event `self.useQuantitySkill`
  ;[1 1 1] call parents to start CD/remove, then call class function to do special power
  (`parent.useQuantitySkill`)
  (`self.useSkillQty`))

(event `self.UseUltimateSkill`
  ;[1 1 1] call parents to start CD/remove, then call class function to do special power
  (`parent.useUltimateSkill`)
  (goto _label))

(event `self.spawnQtySkill`
  ;[1 1 1] call parents to start CD/remove, then call class function to do special power
  (`self.spawnMyQtySkill`))

(event `self.incrementPassiveSkill`
  ;[1 1 1] call parents to start CD/remove, then call class function to do special power
  (`self.incrementMyPassiveSkill`))

(event `self.deactivateSecSkill`
  ;[1 1 1] call parents to start CD/remove, then call class function to do special power
  (`self.deactivateMySecSkill`))

(event `self.deactivateUltSkill`
  ;[1 1 1] call parents to start CD/remove, then call class function to do special power
  (`self.deactiveMyUltSkill`))

(event `self.ReceiveTick`
  (params (DeltaSeconds :type "Float (single-precision)"))
  (`parent.ReceiveTick` DeltaSeconds))

(event `self.ReceiveBeginPlay`
  (bind _returnvalue (`SceneComponent.K2_GetComponentToWorld` (`self.Mesh`)))
  (bind _returnvalue_2 (`|SpawnActorFromClass` "/Game/BluePrints/Game_BPs/Guns/TEST_ACTOR_GUN.TEST_ACTOR_GUN_C" _returnvalue "Undefined" "OverrideRootScale" null null))
  (bind _returnvalue_3 (`|SpawnActorFromClass` "/Game/BluePrints/Game_BPs/Guns/TEST_ACTOR_GUN1.TEST_ACTOR_GUN1_C" _returnvalue "Undefined" "OverrideRootScale" null null))
  (bind _returnvalue_4 (`|SpawnActorFromClass` "/Game/BluePrints/Game_BPs/Guns/TEST_ACTOR_GUN2.TEST_ACTOR_GUN2_C" _returnvalue "Undefined" "OverrideRootScale" null null))
  (`self.createBaseGun` _returnvalue_2 (`/Game/BluePrints/Game_BPs/Guns/TEST_ACTOR_GUN.ProjectilePointSpawn` _returnvalue_2) _returnvalue_3 (`/Game/BluePrints/Game_BPs/Guns/TEST_ACTOR_GUN1.ProjectilePointSpawn` _returnvalue_3) _returnvalue_4)
  (`parent.ReceiveBeginPlay`))

(fn `deactivateMySecSkill`
  (set `self.b_IsAdrenalineBoosted` false))

(fn `deactiveMyUltSkill`)

(fn `incrementMyPassiveSkill`
  ;[1 1 1] add 5% health on kill, stay in range 0 to max health
  (bind _outactors (`GameplayStatics.GetAllActorsWithTag` "friendly"))
  (for _array_element _outactors
    (bind _asbp_parent_chr (cast `/Game/BluePrints/Game_BPs/BP_ParentChr` _array_element))
    (bind _int_actualhealth (`/Game/BluePrints/Game_BPs/BP_ParentChr.int_actualHealth` _asbp_parent_chr))
    (bind _max_health (`/Game/BluePrints/Game_BPs/BP_ParentChr.MAX_HEALTH` _asbp_parent_chr))
    (if (< _int_actualhealth _max_health)
      (bind _returnvalue (+ _int_actualhealth (`KismetMathLibrary.FTrunc` (/ (* _max_health 5.0) 100.0))))
      (if (> _returnvalue _max_health)
        (set `/Game/BluePrints/Game_BPs/BP_ParentChr.int_actualHealth` _max_health _asbp_parent_chr)
        (else
          (set `/Game/BluePrints/Game_BPs/BP_ParentChr.int_actualHealth` _returnvalue _asbp_parent_chr))))))

(fn `spawnMyQtySkill`
  (bind _mesh (`self.Mesh`))
  (`|SpawnActorFromClass` (`self.RefQtySkillGrenade`) (`KismetMathLibrary.MakeTransform` (`SceneComponent.GetSocketLocation` _mesh "S_Active_Weapon") (`SceneComponent.GetSocketRotation` _mesh "S_Active_Weapon")) "Undefined" "OverrideRootScale" null null))

(fn `UserConstructionScript`)

(fn `useSkillPrimary`
  (`/Engine/EditorBlueprintResources/ActorMacros.Switch Has Authority`
    (:`Authority`
      (`|SpawnActorFromClass` "/Game/BluePrints/Game_BPs/Guns/A_Heal_Projectile.A_Heal_Projectile_C" (`SceneComponent.K2_GetComponentToWorld` (`/Game/BluePrints/Game_BPs/CBP_Active_Gun.WeaponArrow` (`self.ActiveWeapon`))) "Undefined" "OverrideRootScale" null null))))

(fn `useSkillQty`
  (`self.PlayAnimMontage` "/Game/BluePrints/Game_BPs/Montage/MT_THROWGRENADE.MT_THROWGRENADE")
  (set `self.flt_timerIsinAction` 1.5)
  (set `self.b_triggerSpawnGrenade` true))

(fn `useSkillSecondary`
  (set `self.flt_timerInUseSecSkill` 5.0)
  (set `self.b_secSkillOn` true)
  (set `self.b_IsAdrenalineBoosted` true))

(fn `useSkillUltimate`
  (bind (_returnvalue_location _returnvalue_rotation _returnvalue_scale) (`KismetMathLibrary.BreakTransform` (`self.GetTransform`)))
  (`/Engine/EditorBlueprintResources/ActorMacros.Switch Has Authority`
    (:`Authority`
      (bind _returnvalue (`|SpawnActorFromClass` "/Game/BluePrints/Game_BPs/SkillsActors/A_MedicUlti.A_MedicUlti_C" (`KismetMathLibrary.MakeTransform` (+ _returnvalue_location (* (`SceneComponent.GetForwardVector` (`self.Mesh`)) 5.0)) _returnvalue_rotation _returnvalue_scale) "Undefined" "OverrideRootScale" null null))
      (`/Game/BluePrints/Game_BPs/SkillsActors/A_MedicUlti.SetTimerTurret` _returnvalue 10.0))))