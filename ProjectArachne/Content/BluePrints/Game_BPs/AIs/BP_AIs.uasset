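; BP_AIs is an AI enemy that tracks players and fires projectiles.
; On server Tick, it counts down an attack cooldown and periodically stores the player with the shortest nav path, considering only those with BIsDying set.
; Pawn sensing keeps the last seen pawn in VisiblePawns, cleared after a retriggerable delay.
; ShootAtTarget spawns a damage-carrying projectile from ShootingArrow when the cooldown expires.
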(event `self.ReceiveTick`
  (params (DeltaSeconds :type "Float (single-precision)"))
  (bind _flt_blackboardupdate (`self.flt_BlackBoardUpdate`))
  (`/Engine/EditorBlueprintResources/ActorMacros.Switch Has Authority`
    (:`Authority`
      (set `self.flt_TimeUpdate` DeltaSeconds)
      (if (not (<= (`self.flt_TimerAttack`) 0.0))
        (set `self.flt_TimerAttack` (- (`self.flt_TimerAttack`) (`self.flt_TimeUpdate`))))
      ;[1 1 1] BlackBoard Update
      (if (> _flt_blackboardupdate 0.0)
        (set `self.flt_BlackBoardUpdate` (- _flt_blackboardupdate (`self.flt_TimeUpdate`)))
        (else
          (set `self.flt_BlackBoardUpdate` 1.0)
          (set `self.PathLenghtToPlayer` 99999.0)
          (for _index (range (`AdvancedSessionsLibrary.GetNumberOfNetworkPlayers`))
            (bind _asbp_parent_chr (cast `/Game/BluePrints/Game_BPs/BP_ParentChr` (`GameplayStatics.GetPlayerCharacter` _index)))
            (if (`/Game/BluePrints/Game_BPs/BP_ParentChr.b_IsDying` _asbp_parent_chr)
              (bind _returnvalue (`NavigationSystem.FindPathToActorSynchronously` (`self.K2_GetActorLocation`) _asbp_parent_chr))
              (bind _returnvalue_2 (`NavigationPath.GetPathLength` _returnvalue))
              (if (and (< _returnvalue_2 (`self.PathLenghtToPlayer`)) (!= _returnvalue_2 -1.0))
                (set `self.ClosesPlayer` _index)
                (set `self.PathLenghtToPlayer` _returnvalue_2))))
          (bind _asbp_parent_chr_2 (cast `/Game/BluePrints/Game_BPs/BP_ParentChr` (`GameplayStatics.GetPlayerCharacter` (`self.ClosesPlayer`))))
          (set `self.ClosestPlayer` _asbp_parent_chr_2))))))

(event `self.PawnSensing.OnSeePawn`
  (params (Pawn :type "Pawn Object Reference"))
  (bind _visible_pawns (`self.Visible Pawns`))
  (`/Engine/EditorBlueprintResources/ActorMacros.Switch Has Authority`
    (:`Authority`
      (`KismetArrayLibrary.Array_Clear` _visible_pawns)
      (`KismetArrayLibrary.Array_Add` _visible_pawns Pawn)
      (`KismetSystemLibrary.RetriggerableDelay` 0.6)
      (`KismetArrayLibrary.Array_Clear` _visible_pawns))))

(fn `ShootAtTarget`
  (`KismetSystemLibrary.PrintString` "PANPAN!")
  (if (<= (`self.flt_TimerAttack`) 0.0)
    (set `self.flt_TimerAttack` (`self.MAX_TIMER_SHOOTING`))
    (`|SpawnActorFromClass` "/Game/BluePrints/Game_BPs/AIs/AI_DistanceProjectile.AI_DistanceProjectile_C" (`SceneComponent.K2_GetComponentToWorld` (`self.ShootingArrow`)) "Undefined" "OverrideRootScale" null (`self.int_DamageDone`) null)))

(fn `UserConstructionScript`)