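; Parent character Blueprint that handles player input for movement stances, camera look and a basic shot.
; Jog, hold or toggle crouch, and prone set state flags and walk speed; prone blocks movement until a delay after standing.
; Jump varies launch velocity when moving, or leaves crouch instead if crouched.
; Shooting fires a short debug-drawn line trace along control rotation, spawning emitter and sound calls at the hit location.
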(event `self.ReceiveBeginPlay`)

(event `InputAction|Jog`
  (params (Key :type "Key Structure"))
  (bind _charactermovement (`self.CharacterMovement`))
  ;[1 1 1] Listener to input(key) JOG, do cases and set JOG
  (:`Pressed`
    (set `self.JogPressed` true)
    (set `CharacterMovementComponent.MaxWalkSpeed` 1000.0 _charactermovement))
  (:`Released`
    (set `self.JogPressed` false)
    (if (`self.CrouchPressed`)
      (set `CharacterMovementComponent.MaxWalkSpeed` 180.0 _charactermovement)
      (else
        (set `CharacterMovementComponent.MaxWalkSpeed` 205.0 _charactermovement)))))

(event `InputAction|Crouch`
  (params (Key :type "Key Structure"))
  (bind _charactermovement (`self.CharacterMovement`))
  ;[1 1 1] Listener to input(key) CROUCH, do cases and set CROUCH
  (:`Pressed`
    (set `self.ShouldTriggerCrouch` false)
    (set `self.CrouchPressed` true)
    (set `CharacterMovementComponent.MaxWalkSpeed` 180.0 _charactermovement))
  (:`Released`
    (set `self.ShouldTriggerCrouch` true)
    (set `self.CrouchPressed` false)
    (if (`self.JogPressed`)
      (set `CharacterMovementComponent.MaxWalkSpeed` 1000.0 _charactermovement)
      (else
        (set `CharacterMovementComponent.MaxWalkSpeed` 205.0 _charactermovement)))))

(event `InputAction|Toggle Crouch`
  (params (Key :type "Key Structure"))
  (bind _charactermovement (`self.CharacterMovement`))
  ;[1 1 1] Listener to input(key) TOGGLE CROUCH, do cases and set CROUCH
  (:`Released`
    (if (`self.PronePressed`) :!label _label
      _
      (elif (`self.ShouldTriggerCrouch`)
        (set `self.CrouchPressed` true)
        (set `self.ShouldTriggerCrouch` false)
        (set `CharacterMovementComponent.MaxWalkSpeed` 180.0 _charactermovement)
        (else
          (set `self.CrouchPressed` false)
          (set `self.ShouldTriggerCrouch` true)
          (if (`self.JogPressed`)
            (set `CharacterMovementComponent.MaxWalkSpeed` 1000.0 _charactermovement)
            (else
              (set `CharacterMovementComponent.MaxWalkSpeed` 205.0 _charactermovement))))))))

(event `InputAction|Jump`
  (params (Key :type "Key Structure"))
  (bind _charactermovement (`self.CharacterMovement`))
  ;[1 1 1] Listener to input(key) JUMP, do cases and set JUMP
  (:`Pressed`
    (if (`NavMovementComponent.IsFlying` (`self.CharacterMovement`))
      _
      (elif (`self.DisableMovement`)
        _
        (elif (`self.CrouchPressed`)
          (goto _label)
          (elif (> (`CharacterMovementComponent.MaxWalkSpeed` (`self.CharacterMovement`)) 160.0)
            (if (> (`KismetMathLibrary.VSize` (`MovementComponent.Velocity` (`self.CharacterMovement`))) 0.0)
              (`self.Jump`)
              (set `CharacterMovementComponent.JumpZVelocity` 365.0 _charactermovement)
              (set `self.JumpPressed` true)
              (else
                (`self.Jump`)
                (set `CharacterMovementComponent.JumpZVelocity` 340.0 _charactermovement)
                (set `self.JumpPressed` true))))))))
  (:`Released`
    (set `self.JumpPressed` false)))

(event `InputAction|Prone`
  (params (Key :type "Key Structure"))
  ;[1 1 1] Listener to input(key) PRONE, do cases and set PRONE
  (:`Pressed`
    (if (not (`self.CrouchPressed`))
      (`/Engine/EditorBlueprintResources/StandardMacros.FlipFlop`
        (:`A`
          (set `self.PronePressed` true)
          (set `self.DisableMovement` true))
        (:`B`
          (set `self.PronePressed` false)
          (`KismetSystemLibrary.Delay` 1.4)
          (set `self.DisableMovement` false))))))

(event `InputAction|Shoot`
  (params (Key :type "Key Structure"))
  (bind _returnvalue (`self.K2_GetActorLocation`))
  (bind _returnvalue_2 (`KismetMathLibrary.MakeVector` (.x _returnvalue) (.y _returnvalue) (+ (.z _returnvalue) 1.0)))
  ;[1 1 1] Listener to input(key) SHOOT, do cases and do SHOOT
  (:`Pressed`
    (`GameplayStatics.PlaySoundAtLocation` null _returnvalue)
    (bind _outhit (`KismetSystemLibrary.LineTraceSingle` :`Start` _returnvalue_2 :`End` (+ _returnvalue_2 (* (`KismetMathLibrary.Conv_RotatorToVector` (`self.GetControlRotation`)) 250.0)) :`TraceChannel` "TraceTypeQuery1" :`DrawDebugType` "ForDuration"))
    (bind (_bblockinghit _binitialoverlap _time _distance _location) (`GameplayStatics.BreakHitResult` _outhit))
    ;;[1 1 1] To add : PARTICLES + SOUNDS AT END LOC OF RAYCAST IF ANY
    (`GameplayStatics.SpawnEmitterAtLocation` null _location)
    (`GameplayStatics.PlaySoundAtLocation` null _location)))

(event `InputAxis|Turn`
  (params (AxisValue :type "Float (single-precision)"))
  ;[1 1 1] Input for movement and view.
  (`self.AddControllerYawInput` AxisValue))

(event `InputAxis|LookUp`
  (params (AxisValue :type "Float (single-precision)"))
  ;[1 1 1] Input for movement and view.
  (`self.AddControllerPitchInput` AxisValue))

(event `InputAxis|MoveForward`
  (params (AxisValue :type "Float (single-precision)"))
  ;[1 1 1] Input for movement and view.
  (if (not (`self.DisableMovement`))
    (`self.AddMovementInput` (`KismetMathLibrary.GetForwardVector` (`KismetMathLibrary.MakeRotator` 0.0 0.0 (.yaw (`self.GetControlRotation`)))) AxisValue)))

(event `InputAxis|MoveRight`
  (params (AxisValue :type "Float (single-precision)"))
  ;[1 1 1] Input for movement and view.
  (if (not (`self.DisableMovement`))
    (`self.AddMovementInput` (`KismetMathLibrary.GetRightVector` (`KismetMathLibrary.MakeRotator` 0.0 0.0 (.yaw (`self.GetControlRotation`)))) AxisValue)))

(fn `UserConstructionScript`)