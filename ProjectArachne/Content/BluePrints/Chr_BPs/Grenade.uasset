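; Grenade actor that goes off on a fixed short timer after spawning.
; On BeginPlay it applies a velocity-based impulse to its mesh, zeroed out by the multiplier, and fires its radial force impulse immediately, before the delay.
; After the delay it spawns a particle effect at its location with a sound attached, then destroys itself.
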(event `self.ReceiveBeginPlay`
  (`PrimitiveComponent.AddImpulseAtLocation` (`self.GrenadeMesh`) (* (`self.GetVelocity`) (0.0 0.0 0.0)) (`self.K2_GetActorLocation`) "None")
  (`RadialForceComponent.FireImpulse` (`self.RadialForce`))
  (`KismetSystemLibrary.Delay` 1.0)
  (bind _returnvalue (`GameplayStatics.SpawnEmitterAtLocation` "/Engine/Tutorial/SubEditors/TutorialAssets/TutorialParticleSystem.TutorialParticleSystem" (`self.K2_GetActorLocation`)))
  (`GameplayStatics.SpawnSoundAttached` "/Engine/EditorSounds/Notifications/CompileStart_Cue.CompileStart_Cue" _returnvalue)
  (`self.K2_DestroyActor`))

(fn `UserConstructionScript`)