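; Engineer character class that overrides the parent character's skill events, calling the parent for cooldowns before applying its own effects.
; BeginPlay spawns test main, sub and melee weapons.
; Skills set parent timers and flags: secondary applies glass materials, ultimate boosts damage, quantity plays a throw montage and flags a socket-spawned grenade.
; The passive cuts "friendly" characters' primary and secondary cooldowns by 10% (commented 20%), skipping secondary when primary clamps to zero.
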(event `self.UsePrimarySkill`
  ;[1 1 1] call parents to start CD/remove, then call class function to do special power
  (`parent.usePrimarySkill`)
  (`self.useSkillPrimary`))

(event `self.UseSecondarySkill`
  ;[1 1 1] call parents to start CD/remove, then call class function to do special power
  (`parent.useSecondarySkill`)
  (`self.useSkillSecondary`))

(event `self.useQuantitySkill`
  ;[1 1 1] call parents to start CD/remove, then call class function to do special power
  (`parent.useQuantitySkill`)
  (`self.useSkillQty`))

(event `self.UseUltimateSkill`
  ;[1 1 1] call parents to start CD/remove, then call class function to do special power
  (`parent.useUltimateSkill`)
  (`self.useSkillUltimate`))

(event `self.spawnQtySkill`
  ;[1 1 1] call parents to start CD/remove, then call class function to do special power
  (`self.spawnMyQtySkill`))

(event `self.incrementPassiveSkill`
  ;[1 1 1] call parents to start CD/remove, then call class function to do special power
  (`self.incrementMyPassiveSkill`))

(event `self.deactivateSecSkill`
  ;[1 1 1] call parents to start CD/remove, then call class function to do special power
  (`self.deactivateMySecSkill`))

(event `self.deactivateUltSkill`
  ;[1 1 1] call parents to start CD/remove, then call class function to do special power
  (`self.deactiveMyUltSkill`))

(event `self.ReceiveTick`
  (params (DeltaSeconds :type "Float (single-precision)"))
  (`parent.ReceiveTick` DeltaSeconds))

(event `self.ReceiveBeginPlay`
  (bind _returnvalue (`SceneComponent.K2_GetComponentToWorld` (`self.Mesh`)))
  (bind _returnvalue_2 (`|SpawnActorFromClass` "/Game/BluePrints/Chr_BPs/GunPlaceHolder/TEST_ACTOR_GUN.TEST_ACTOR_GUN_C" _returnvalue "Undefined" "OverrideRootScale" null null))
  (bind _returnvalue_3 (`|SpawnActorFromClass` "/Game/BluePrints/Chr_BPs/GunPlaceHolder/TEST_ACTOR_GUN1.TEST_ACTOR_GUN1_C" _returnvalue "Undefined" "OverrideRootScale" null null))
  (bind _returnvalue_4 (`|SpawnActorFromClass` "/Game/BluePrints/Chr_BPs/GunPlaceHolder/TEST_ACTOR_GUN2.TEST_ACTOR_GUN2_C" _returnvalue "Undefined" "OverrideRootScale" null null))
  (`self.createBaseGun` _returnvalue_2 (`/Game/BluePrints/Chr_BPs/GunPlaceHolder/TEST_ACTOR_GUN.ProjectilePointSpawn` _returnvalue_2) _returnvalue_3 (`/Game/BluePrints/Chr_BPs/GunPlaceHolder/TEST_ACTOR_GUN1.ProjectilePointSpawn` _returnvalue_3) _returnvalue_4)
  (`parent.ReceiveBeginPlay`))

(fn `deactivateMySecSkill`
  (bind _mesh (`self.Mesh`))
  (`PrimitiveComponent.SetMaterial` _mesh 0 "/Game/Animations/AnimStarterPack/UE4_Mannequin/Materials/M_UE4Man_Body.M_UE4Man_Body")
  (`PrimitiveComponent.SetMaterial` _mesh 1 "/Game/Animations/AnimStarterPack/UE4_Mannequin/Materials/M_UE4Man_ChestLogo.M_UE4Man_ChestLogo"))

(fn `deactiveMyUltSkill`
  (set `self.flt_boostTotalDamage` 0.0))

(fn `incrementMyPassiveSkill`
  ;[1 1 1] Remove 20% of CD
  (bind _outactors (`GameplayStatics.GetAllActorsWithTag` "friendly"))
  (for _array_element _outactors
    (bind _asbp_parent_chr (cast `/Game/BluePrints/Chr_BPs/BP_ParentChr` _array_element))
    (bind _flt_timerprimaryskill (`/Game/BluePrints/Chr_BPs/BP_ParentChr.flt_timerPrimarySkill` _asbp_parent_chr))
    (if (> _flt_timerprimaryskill 0.0)
      (bind _returnvalue (- _flt_timerprimaryskill (/ (* (`/Game/BluePrints/Chr_BPs/BP_ParentChr.MAX_TIMER_PRIMARY_SKILL` _asbp_parent_chr) 10.0) 100.0)))
      (if (< _returnvalue 0.0)
        (set `/Game/BluePrints/Chr_BPs/BP_ParentChr.flt_timerPrimarySkill` 0.0 _asbp_parent_chr)
        (else
          (set `/Game/BluePrints/Chr_BPs/BP_ParentChr.flt_timerPrimarySkill` _returnvalue _asbp_parent_chr)
          (bind _flt_timersecondaryskill (`/Game/BluePrints/Chr_BPs/BP_ParentChr.flt_timerSecondarySkill` _asbp_parent_chr))
          (if (> _flt_timersecondaryskill 0.0) :!label _label
            (bind _returnvalue_2 (- _flt_timersecondaryskill (/ (* (`/Game/BluePrints/Chr_BPs/BP_ParentChr.MAX_TIMER_SECONDARY_SKILL` _asbp_parent_chr) 10.0) 100.0)))
            (if (< _returnvalue_2 0.0)
              (set `/Game/BluePrints/Chr_BPs/BP_ParentChr.flt_timerSecondarySkill` 0.0 _asbp_parent_chr)
              (else
                (set `/Game/BluePrints/Chr_BPs/BP_ParentChr.flt_timerSecondarySkill` _returnvalue_2 _asbp_parent_chr))))))
      (else
        (goto _label)))))

(fn `spawnMyQtySkill`
  (bind _mesh (`self.Mesh`))
  (`|SpawnActorFromClass` (`self.RefQtySkillGrenade`) (`KismetMathLibrary.MakeTransform` (`SceneComponent.GetSocketLocation` _mesh "S_Active_Weapon") (`SceneComponent.GetSocketRotation` _mesh "S_Active_Weapon")) "Undefined" "OverrideRootScale" null null))

(fn `UserConstructionScript`)

(fn `useSkillPrimary`
  (set `self.flt_timerInUsePrimSkill` 5.0)
  (set `self.b_primSkillOn` true))

(fn `useSkillQty`
  (`self.PlayAnimMontage` "/Game/BluePrints/Chr_BPs/Montage/MT_THROWGRENADE.MT_THROWGRENADE")
  (set `self.flt_timerIsinAction` 1.5)
  (set `self.b_triggerSpawnGrenade` true))

(fn `useSkillSecondary`
  (bind _mesh (`self.Mesh`))
  (set `self.flt_timerInUseSecSkill` 5.0)
  (set `self.b_secSkillOn` true)
  (`PrimitiveComponent.SetMaterial` _mesh 0 "/Game/Materials/Glass.Glass")
  (`PrimitiveComponent.SetMaterial` _mesh 1 "/Game/Materials/Glass.Glass"))

(fn `useSkillUltimate`
  (set `self.b_ultSkillOn` true)
  (set `self.flt_timerInUseUltSkill` 10.0)
  (set `self.flt_boostTotalDamage` 50.0))