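; Gun projectile that damages what it hits, using data from the gun that fired it, stored through SetActiveGun.
; On Hit, IDamageable targets receive the gun's damage through an interface message, unless the Friendly tag check passes, which plays a fixed explosion and sound instead.
; Other surfaces get the gun's touch particle and sound.
; The projectile destroys itself in every case.
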(event `self.ReceiveHit`
  (params (MyComp :type "PrimitiveComponent Object Reference") (Other :type "Actor Object Reference") (OtherComp :type "PrimitiveComponent Object Reference") (bSelfMoved :type Boolean) (HitLocation :type "Vector Structure") (HitNormal :type "Vector Structure") (NormalImpulse :type "Vector Structure") (Hit :type "HitResult Structure (by ref)"))
  ;[1 1 1] PARTICLES + SOUNDS AT CONTACT
  (if (`KismetSystemLibrary.DoesImplementInterface` Other "/Game/BluePrints/Chr_BPs/iDamageable.iDamageable_C")
    (if (not (`self.ActorHasTag` "Friendly"))
      (message `/Game/BluePrints/Chr_BPs/iDamageable.AffectHealth` Other (`/Game/BluePrints/Chr_BPs/Active_Gun_BP.flt_damage` (`self.ActiveGun`)))
      (`self.K2_DestroyActor`)
      (else
        ;;[1 1 1] Projectile hit friendly
        (`GameplayStatics.SpawnEmitterAtLocation` "/Game/Particles/P_Logo_Flare.P_Explosion" HitLocation)
        (`GameplayStatics.PlaySoundAtLocation` "/Engine/EditorSounds/GamePreview/EndSimulate_Cue.EndSimulate_Cue" HitLocation)
        (`self.K2_DestroyActor`)))
    (else
      ;;[1 1 1] Projectile hit decors
      (`GameplayStatics.SpawnEmitterAtLocation` (`/Game/BluePrints/Chr_BPs/Active_Gun_BP.TouchParticle` (`self.ActiveGun`)) HitLocation)
      (`GameplayStatics.PlaySoundAtLocation` (`/Game/BluePrints/Chr_BPs/Active_Gun_BP.TouchSound` (`self.ActiveGun`)) HitLocation)
      (`self.K2_DestroyActor`))))

(fn `setActiveGun`
  (params (ActiveGunWhenShot :type "/Game/BluePrints/Chr_BPs/Active_Gun_BP Object Reference (by ref)"))
  (set `self.ActiveGun` ActiveGunWhenShot))

(fn `UserConstructionScript`)